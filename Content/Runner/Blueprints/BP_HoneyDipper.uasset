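; BP_HoneyDipper is a runner-game pickup that grants a super speed boost.
; On BeginPlay it stores its height and destroys any BP_Coin actors within a small surrounding sphere, clearing its spot.
; Tick bobs it vertically on a sine wave around that height.
; When a BP_RunnerCharacter interacts, it activates GA_SuperSpeed through the character's Ability System Component and destroys itself.
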(event `self.ReceiveBeginPlay`
  (bind (_returnvalue_x _returnvalue_y _returnvalue_z) (`KismetMathLibrary.BreakVector` (`self.K2_GetActorLocation`)))
  (set `self.Initial Z` _returnvalue_z)
  (bind _outactors (`KismetSystemLibrary.SphereOverlapActors` (`self.K2_GetActorLocation`) 150.0 (`|MakeArray` "ObjectTypeQuery9" :!type "EObjectTypeQuery Enum") "/Game/Runner/Blueprints/BP_Coin.BP_Coin_C"))
  (bind (_arrayindex _arrayelement) (`/Engine/EditorBlueprintResources/StandardMacros.ReverseForEachLoop` _outactors)
    (:`LoopBody`
      (`self.K2_DestroyActor` _arrayelement))))

(event `self.ReceiveTick`
  (params (DeltaSeconds :type "Float (single-precision)"))
  (bind (_returnvalue_x _returnvalue_y) (`KismetMathLibrary.BreakVector` (`self.K2_GetActorLocation`)))
  (bind _output_get (set `self.Total Seconds` (+ (* DeltaSeconds 200.0) (`self.Total Seconds`))))
  (`self.K2_SetActorLocation` (`KismetMathLibrary.MakeVector` _returnvalue_x _returnvalue_y (+ (* (`KismetMathLibrary.DegSin` _output_get) 25.0) (`self.Initial Z`)))))

(event `self.Interact`
  (params (`Interacting Actor` :type "Actor Object Reference"))
  (bind _asbp_runner_character (cast `/Game/Runner/Blueprints/BP_RunnerCharacter` `Interacting Actor`))
  (`AbilitySystemComponent.TryActivateAbilityByClass` (`AbilitySystemBlueprintLibrary.GetAbilitySystemComponent` _asbp_runner_character) "/Game/Runner/Blueprints/GA_SuperSpeed.GA_SuperSpeed_C" true)
  (`self.K2_DestroyActor`))

(fn `UserConstructionScript`)