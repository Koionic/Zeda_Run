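; BP_ParticleFollower is a runner effect actor that shows a Niagara effect while the player has super speed.
; On BeginPlay it stores its starting height and starts async gameplay tag listeners on the player pawn.
; Adding Runner.SuperSpeed activates the effect and removing it deactivates it, despite the event being named MagnetFX.
; Tick keeps the actor's current X and Y but locks Z to the starting height.
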(event `Magnet FX`
  (bind _returnvalue (`GameplayStatics.GetPlayerPawn` 0))
  (bind _niagara (`self.Niagara`))
  (`AbilityAsync_WaitGameplayTagAdded.WaitGameplayTagAddToActor` _returnvalue (struct :`TagName` "Runner.SuperSpeed")
    (:`then`
      (`AbilityAsync_WaitGameplayTagRemoved.WaitGameplayTagRemoveFromActor` _returnvalue (struct :`TagName` "Runner.SuperSpeed")
        (:`Removed`
          (`ActorComponent.Deactivate` _niagara))))
    (:`Added`
      (`ActorComponent.Activate` _niagara false))))

(event `self.ReceiveBeginPlay`
  (bind (_returnvalue_x _returnvalue_y _returnvalue_z) (`KismetMathLibrary.BreakVector` (`self.K2_GetActorLocation`)))
  (set `self.Initial Z` _returnvalue_z)
  (`self.Magnet FX`))

(event `self.ReceiveTick`
  (params (DeltaSeconds :type "Float (single-precision)"))
  (bind (_returnvalue_x _returnvalue_y) (`KismetMathLibrary.BreakVector` (`self.K2_GetActorLocation`)))
  (`self.K2_SetActorLocation` (`KismetMathLibrary.MakeVector` _returnvalue_x _returnvalue_y (`self.Initial Z`))))

(fn `UserConstructionScript`)