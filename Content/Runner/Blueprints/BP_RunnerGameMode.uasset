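; Game mode for an endless runner that manages world speed, score, coins and a rolling chain of floor tiles.
; On BeginPlay it seeds the floor chain, shows the gameplay widget, loads saved coins and binds to the player's death.
; ExtendFloor spawns tiles from the last tile's attach points and destroys the oldest beyond the limit.
; Death saves score and coins; the pause and game-over sequence is unconnected.
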(event `self.ReceiveBeginPlay`
  (add `/Game/Runner/Blueprints/BP_RunnerCharacter.OnDie` (`/Game/Runner/Functions/BPFL_CoreFunctions.Get Runner Player`) (delegate `On Character Death`))
  (set `self.Current World Speed` (`self.Starting World Speed`))
  (`self.Set Up Floors`)
  (bind _returnvalue (`|CreateWidget` "/Game/Runner/HUD/WBP_Gameplay.WBP_Gameplay_C"))
  (`UserWidget.AddToViewport` _returnvalue 0)
  (bind (_success _value) (`/Game/Runner/Functions/BPFL_CoreFunctions.Get Save Value` "CoinValue"))
  (if _success
    (set `self.Coins` _value)))

(event `On Character Death`
  (`self.Save Stats`))

(fn `AddFloor`
  (bind _floor_tiles (`self.Floor Tiles`))
  (bind (_tilespawnpoint_location _tilespawnpoint_rotation _tilespawnpoint_scale) (`KismetMathLibrary.BreakTransform` (`self.TileSpawnPoint`)))
  (bind _output (`|GetArrayItem` _floor_tiles (`KismetArrayLibrary.Array_LastIndex` _floor_tiles)))
  (bind (_front_attach_point _back_attach_point) (`/Game/Runner/Blueprints/BP_Floor.Get Attach Points` _output))
  (`/Engine/EditorBlueprintResources/StandardMacros.IsValid` _output
    (:`Is Valid`
      (set `self.TileSpawnPoint` _front_attach_point))
    (:`Is Not Valid`
      _))
  (`KismetSystemLibrary.PrintString` "Spawn Start")
  (bind _returnvalue (`|SpawnActorFromClass` "/Game/Runner/Blueprints/BP_Floor.BP_Floor_C" (`KismetMathLibrary.MakeTransform` (- _tilespawnpoint_location (`KismetMathLibrary.InverseTransformLocation` (`self.GetTransform` _output) (.location _back_attach_point))) _tilespawnpoint_rotation _tilespawnpoint_scale) "AlwaysSpawn" "MultiplyWithRoot" null null))
  (`KismetSystemLibrary.PrintString` "Spawn End")
  (`KismetArrayLibrary.Array_Add` (`self.Floor Tiles`) _returnvalue)
  (`/Engine/EditorBlueprintResources/StandardMacros.IncrementInt` (`self.Floor Count`)
    (:`  `
      (`/Engine/EditorBlueprintResources/StandardMacros.IncrementInt` (`self.Floor Count Until Moving Obstacle`)))))

(fn `Extend Floor`
  (bind _floor_tiles (`self.Floor Tiles`))
  (bind _output (`|GetArrayItem` _floor_tiles))
  (`self.AddFloor`)
  (if (> (`KismetArrayLibrary.Array_Length` (`self.Floor Tiles`)) (+ (`self.Number Of Tiles`) 1))
    ;[1 1 1] Destroy Oldest Floor Tile
    (`self.K2_DestroyActor` _output)
    (`KismetArrayLibrary.Array_RemoveItem` _floor_tiles _output)))

(fn `Increase Score`
  (set `self.Current Points` (+ (* (`self.Points Mulit`) 1) (`self.Current Points`))))

(fn `Save Stats`
  (`/Game/Runner/Functions/BPFL_CoreFunctions.Save Stat` "HighScoreValue" (`self.Current Points`))
  (`/Game/Runner/Functions/BPFL_CoreFunctions.Save Stat` "CoinValue" (`self.Coins`)))

(fn `Set Up Floors`
  (bind _returnvalue (`GameplayStatics.GetActorOfClass` "/Game/Runner/Blueprints/BP_Floor.BP_Floor_C"))
  (`/Engine/EditorBlueprintResources/StandardMacros.IsValid` _returnvalue
    (:`Is Valid`
      (`KismetArrayLibrary.Array_Add` (`self.Floor Tiles`) _returnvalue))
    (:`Is Not Valid`
      _))
  (for _ (range (`KismetArrayLibrary.Array_Length` (`self.Floor Tiles`)) (+ (- (`self.Number Of Tiles`) 3) 1))
    (`self.AddFloor`)))

(fn `UserConstructionScript`)