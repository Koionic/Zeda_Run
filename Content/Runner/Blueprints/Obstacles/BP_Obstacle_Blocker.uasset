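; BP_Obstacle_Blocker is a runner obstacle that kills the player on contact unless they are sliding.
; On actor overlap it calls the parent handler, casts the other actor to BP_RunnerCharacter, and calls Die when IsSliding is false.
; BeginPlay and Tick are disabled, and the construction script only calls its parent.
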(event `self.ReceiveActorBeginOverlap`
  (params (OtherActor :type "Actor Object Reference"))
  (`parent.ReceiveActorBeginOverlap` OtherActor)
  (bind _asbp_runner_character (cast `/Game/Runner/Blueprints/BP_RunnerCharacter` OtherActor))
  (if (not (`/Game/Runner/Blueprints/BP_RunnerCharacter.Is Sliding` _asbp_runner_character))
    (`/Game/Runner/Blueprints/BP_RunnerCharacter.Die` _asbp_runner_character)))

(fn `UserConstructionScript`
  (`parent.UserConstructionScript`))