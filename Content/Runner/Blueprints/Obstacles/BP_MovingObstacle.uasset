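; BP_MovingObstacle is a runner-game obstacle that travels along negative X and kills the player on contact.
; BeginPlay caches the mesh's spawn position and the game mode's world speed once.
; Tick moves it without sweep at world speed times TravelSpeed, holding Y and Z at spawn values.
; Collision overlap calls KillPlayer on the runner character, passing a computed closest bone and a backward X vector.
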(event `self.ReceiveBeginPlay`
  (`parent.ReceiveBeginPlay`)
  (`KismetSystemLibrary.PrintString` "Begin")
  (set `self.Spawn Position` (`SceneComponent.K2_GetComponentLocation` (`self.StaticMesh`)))
  (set `self.World Speed` (`/Game/Runner/Blueprints/BP_RunnerGameMode.Current World Speed` (`/Game/Runner/Functions/BPFL_CoreFunctions.Get Runner Game Mode`))))

(event `self.ReceiveTick`
  (params (DeltaSeconds :type "Float (single-precision)"))
  (bind _returnvalue_x (`KismetMathLibrary.BreakVector` (`self.K2_GetActorLocation`)))
  (bind (_spawn_position_x _spawn_position_y _spawn_position_z) (`KismetMathLibrary.BreakVector` (`self.Spawn Position`)))
  (`parent.ReceiveTick` DeltaSeconds)
  (`self.K2_SetActorLocation` (`KismetMathLibrary.MakeVector` (+ (* DeltaSeconds (* (`self.World Speed`) (`self.Travel Speed`) -1.0)) _returnvalue_x) _spawn_position_y _spawn_position_z)))

(event `self.Collision.OnComponentBeginOverlap`
  (params (OverlappedComponent :type "PrimitiveComponent Object Reference") (OtherActor :type "Actor Object Reference") (OtherComp :type "PrimitiveComponent Object Reference") (OtherBodyIndex :type Integer) (bFromSweep :type Boolean) (SweepResult :type "HitResult Structure (by ref)"))
  (bind _asbp_runner_character (cast `/Game/Runner/Blueprints/BP_RunnerCharacter` OtherActor))
  (`/Game/Runner/Blueprints/BP_RunnerCharacter.KillPlayer` _asbp_runner_character (`|MakeArray` (make `/Game/Runner/Structs/FImpactPoints` (`.ReturnValue` (`SkinnedMeshComponent.FindClosestBone_K2` (`Character.Mesh` _asbp_runner_character) (+ SweepResult_ImpactPoint (`SceneComponent.K2_GetComponentLocation` (`self.StaticMesh`))) 0.0 false)) (-500.0 0.0 0.0)) (struct) :!type "/Game/Runner/Structs/FImpactPoints Structure")))

(fn `UserConstructionScript`
  (`parent.UserConstructionScript`))