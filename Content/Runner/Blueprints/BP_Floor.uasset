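; Floor tile for an endless runner that fills itself with obstacles, coins and power-ups, except on the first tile.
; On BeginPlay it builds per-lane arrow-component spawn points, then shuffles them to place child actors at random.
; Game mode counters gate periodic power-ups and occasional Bee moving obstacles, which spawn as separate actors.
; The runner's first overlap with its collision tells the game mode to extend the floor and increase the score.
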(event `self.ReceiveBeginPlay`
  (bind _asbp_runner_game_mode (cast `/Game/Runner/Blueprints/BP_RunnerGameMode` (`GameplayStatics.GetGameMode`)))
  (set `self.BP Runner Game Mode` _asbp_runner_game_mode)
  (if (not (`self.bFirstTile`))
    (`self.Setup Spawn Points`)
    (`self.Spawn Obstacle`)
    (`self.Set Up Coin Points`)
    (`self.Spawn Coins`)
    (`self.Set Up Power Up Points`)
    (`self.Spawn Power Ups`)))

(event `self.Collision.OnComponentBeginOverlap`
  (params (OverlappedComponent :type "PrimitiveComponent Object Reference") (OtherActor :type "Actor Object Reference") (OtherComp :type "PrimitiveComponent Object Reference") (OtherBodyIndex :type Integer) (bFromSweep :type Boolean) (SweepResult :type "HitResult Structure (by ref)"))
  (cast `/Game/Runner/Blueprints/BP_RunnerCharacter` OtherActor)
  (`/Engine/EditorBlueprintResources/StandardMacros.DoOnce` false
    (:`Completed`
      (`/Game/Runner/Blueprints/BP_RunnerGameMode.Extend Floor` (`self.BP Runner Game Mode`))
      (`/Game/Runner/Blueprints/BP_RunnerGameMode.Increase Score` (`/Game/Runner/Functions/BPFL_CoreFunctions.Get Runner Game Mode`)))))

(fn `Get Attach Points`
  (returns (`Front Attach Point` :type "Transform Structure") (`Back Attach Point` :type "Transform Structure"))
  (return (`SceneComponent.K2_GetComponentToWorld` (`self.Front Attach Point`)) (`SceneComponent.K2_GetComponentToWorld` (`self.Back Attach Point`))))

(fn `Set Up Coin Points`
  (for _array_element (`self.Lane Positions`)
    (for _index (range 10)
      (bind _returnvalue (`AddComponent|NODE_AddArrowComponent-1` :`RelativeTransform` (`KismetMathLibrary.MakeTransform` (`KismetMathLibrary.MakeVector` (* _index 75.0) _array_element))))
      (`ArrowComponent.SetArrowColor` _returnvalue (struct :`R` 1.0 :`G` 0.859946 :`A` 1.0))
      (`KismetArrayLibrary.Array_Add` (`self.Coin Spawn Points`) (`SceneComponent.K2_GetComponentToWorld` _returnvalue)))))

(fn `Set Up Power Up Points`
  (for _array_element (`self.Lane Positions`)
    (for _index (range 1 3)
      (bind _returnvalue (`AddComponent|NODE_AddArrowComponent-2` :`RelativeTransform` (`KismetMathLibrary.MakeTransform` (`KismetMathLibrary.MakeVector` (* _index 200.0) _array_element))))
      (`ArrowComponent.SetArrowColor` _returnvalue (struct :`G` 1.0 :`B` 0.16855 :`A` 1.0))
      (`KismetArrayLibrary.Array_Add` (`self.Power Up Spawn Points`) (`SceneComponent.K2_GetComponentToWorld` _returnvalue)))))

(fn `Setup Spawn Points`
  (for _array_element (`self.Lane Positions`)
    (bind _returnvalue (`AddComponent|NODE_AddArrowComponent-0` :`RelativeTransform` (`KismetMathLibrary.MakeTransform` (`KismetMathLibrary.MakeVector` 0.0 _array_element))))
    (`KismetArrayLibrary.Array_Add` (`self.Spawn Points`) (`SceneComponent.K2_GetComponentToWorld` _returnvalue))))

(fn `Spawn Coins`
  (locals (`Random Spawn Points` :type "Array of Transform Structure"))
  (bind _output_get (set `local.Random Spawn Points` (`self.Coin Spawn Points`)))
  (`KismetArrayLibrary.Array_Shuffle` _output_get)
  (for _index (range (+ (`KismetMathLibrary.RandomIntegerInRange` 5 9) 1))
    (`AddComponent|NODE_AddChildActorComponent-7` :`RelativeTransform` (`KismetMathLibrary.MakeRelativeTransform` (`|GetArrayItem` (`local.Random Spawn Points`) _index) (`self.GetTransform`)))))

(fn `Spawn Moving Obstacle`
  (params (Selection :type Integer) (RelativeTransform :type "Transform Structure"))
  (bind _asbp_runner_game_mode (cast `/Game/Runner/Blueprints/BP_RunnerGameMode` (`GameplayStatics.GetGameMode`)))
  (if (> (`/Game/Runner/Blueprints/BP_RunnerGameMode.Floor Count Until Moving Obstacle` _asbp_runner_game_mode) (`KismetMathLibrary.RandomIntegerInRange` 10 20))
    (switch `int` Selection
      (:`0`
        (`KismetSystemLibrary.PrintString` "Bee")
        (`|SpawnActorFromClass` "/Game/Runner/Blueprints/Obstacles/BP_Bee.BP_Bee_C" (`KismetMathLibrary.MakeTransform` (+ (.location RelativeTransform) (`SceneComponent.K2_GetComponentLocation` (`self.Floor`)))) "AlwaysSpawn" "MultiplyWithRoot" null null)
        (set `/Game/Runner/Blueprints/BP_RunnerGameMode.Floor Count Until Moving Obstacle` 0 _asbp_runner_game_mode)))))

(fn `Spawn Obstacle`
  (locals (`Random Spawn Points` :type "Array of Transform Structure"))
  (bind _output_get (set `local.Random Spawn Points` (`self.Spawn Points`)))
  (`KismetArrayLibrary.Array_Shuffle` _output_get)
  (for _index (range (+ (`KismetMathLibrary.RandomIntegerInRange` 0 2) 1))
    (switch `int` (`KismetMathLibrary.RandomIntegerInRange` 0 2)
      (:`0`
        (bind _returnvalue (`KismetMathLibrary.MakeRelativeTransform` (`|GetArrayItem` (`local.Random Spawn Points`) _index) (`self.GetTransform`)))
        (`AddComponent|NODE_AddChildActorComponent-0` :`RelativeTransform` _returnvalue))
      (:`1`
        (`AddComponent|NODE_AddChildActorComponent-1` :`RelativeTransform` _returnvalue))
      (:`2`
        (`self.Spawn Moving Obstacle` 0 _returnvalue)))))

(fn `Spawn Power Ups`
  (locals (`Random Spawn Points` :type "Array of Transform Structure"))
  (if (== (mod (`/Game/Runner/Blueprints/BP_RunnerGameMode.Floor Count` (`/Game/Runner/Functions/BPFL_CoreFunctions.Get Runner Game Mode`)) (`self.Magnet Spawn Rate`)) 0)
    (bind _output_get (set `local.Random Spawn Points` (`self.Power Up Spawn Points`)))
    (`KismetArrayLibrary.Array_Shuffle` _output_get)
    (`AddComponent|NODE_AddChildActorComponent-8` :`RelativeTransform` (`KismetMathLibrary.MakeRelativeTransform` (`|GetArrayItem` (`local.Random Spawn Points`)) (`self.GetTransform`)))))

(fn `UserConstructionScript`)